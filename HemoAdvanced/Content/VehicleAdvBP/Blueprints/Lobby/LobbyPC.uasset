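; Lobby player controller that shows the lobby menu and passes this player's settings to the game mode.
; Setup events create the menu widget and send settings to LobbyGM through SwapTeam, always with team 0.
; AddPlayerInfo rebuilds the menu's player list from the connected players' info, and EndPlay destroys the session.
; Save check, loading scene, player count update and PlayerSettings OnRep are empty stubs.
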(event `InitialSetup`
  ;[1 1 1] Initial Setup
  (`self.SaveGameCheck`)
  (`self.CallUpdate` (`self.PlayerSettings`)))

(event `SetupLobbyMenu`
  (params (NewParam2 :type "/Game/VehicleAdvBP/Blueprints/AllLevels/PlayerInfo Structure"))
  ;[1 1 1] Setup Lobby Menu
  (set `self.bShowMouseCursor` false)
  (bind _returnvalue (`|CreateWidget` "/Game/UI/Lobby/LobbyMenu.LobbyMenu_C"))
  (bind _output_get (set `self.LobbyMenuWB` _returnvalue))
  (`UserWidget.AddToViewport` _output_get 0)
  (`WidgetBlueprintLibrary.SetInputMode_GameAndUIEx` self _output_get))

(event `CallUpdate`
  (params (PlayerInfo :type "/Game/VehicleAdvBP/Blueprints/AllLevels/PlayerInfo Structure") (ChangeStatus :type Boolean))
  (set `self.PlayerSettings` PlayerInfo)
  (bind _aslobby_gm (cast `/Game/VehicleAdvBP/Blueprints/Lobby/LobbyGM` (`GameplayStatics.GetGameMode`)))
  (`/Game/VehicleAdvBP/Blueprints/Lobby/LobbyGM.SwapTeam` _aslobby_gm null 0 ChangeStatus))

(event `AddPlayerInfo`
  (params (ConnectedPlayerInfo :type "Array of /Game/VehicleAdvBP/Blueprints/AllLevels/PlayerInfo Structure"))
  (bind _lobbymenuwb (`self.LobbyMenuWB`))
  (set `self.AllPlayerInfo` ConnectedPlayerInfo)
  (`/Engine/EditorBlueprintResources/StandardMacros.IsValid` _lobbymenuwb
    (:`Is Valid`
      (`/Game/UI/Lobby/LobbyMenu.ClearPlayeList` _lobbymenuwb)
      (for _array_element (`self.AllPlayerInfo`)
        (`/Game/UI/Lobby/LobbyMenu.UpdatePlayerWindow` (`self.LobbyMenuWB`) _array_element)))))

(event `UpdateNumberOfPlayers`
  (params (`Current Players` :type Integer) (`Max Players` :type Integer))
  (`/Engine/EditorBlueprintResources/StandardMacros.IsValid` (`self.LobbyMenuWB`)))

(event `ShowLoadingScene`)

(event `self.ReceiveEndPlay`
  (params (EndPlayReason :type "EEndPlayReason Enum" :default "Destroyed"))
  (`DestroySessionCallbackProxy.DestroySession` null))

(fn `OnRep_PlayerSettings`)

(fn `SaveGameCheck`)

(fn `UserConstructionScript`)