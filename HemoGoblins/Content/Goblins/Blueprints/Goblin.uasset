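; Goblin character Blueprint that handles the goblin's reaction to being hit.
; The Hit event sets a hit flag, detaches the controller and changes the Collider's tick interval.
; It then attaches a scaled-down blood particle effect to the skeletal mesh and spawns a decal actor at the goblin's X/Y position with a fixed height.
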(event `Hit`
  (set `self.isGetHit?` true)
  (`self.DetachFromControllerPendingDestroy`)
  (`ActorComponent.SetComponentTickInterval` (`self.Collider`) 0.05)
  (`|ExecutionSequence`
    (:`then_0`
      (`GameplayStatics.SpawnEmitterAttached` "/Game/Particles/Blood.Blood" (`self.SkeletalMesh`) "None" (0.0 0.0 0.0) (struct) (0.5 0.5 0.5)))
    (:`then_1`
      (`|SpawnActorFromClass` "/Game/Goblins/Blueprints/Decal_BP.Decal_BP_C" (`KismetMathLibrary.MakeTransform` (`KismetMathLibrary.MakeVector` (.x (`self.K2_GetActorLocation`)) (.y (`self.K2_GetActorLocation`)) 110.0)) "Undefined" "OverrideRootScale" null null)
      (`/Engine/EditorBlueprintResources/StandardMacros.DoOnce` false))))

(fn `UserConstructionScript`)