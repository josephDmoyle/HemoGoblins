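; Goblin spawn manager that periodically spawns a Goblin at a random entry from its SpawnPoint array.
; Tick sets its own interval to a couple of seconds, then spawns at that point's transform, adjusting for collisions or skipping the spawn if still blocked.
; The MaxSpawn check and count printout are disconnected, so spawning is uncapped and nothing here adds to SpawnedArray.
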(event `self.ReceiveTick`
  (params (DeltaSeconds :type "Float (single-precision)"))
  (`self.SetActorTickInterval` 2.0)
  (`|SpawnActorFromClass` "/Game/Goblins/Blueprints/Goblin.Goblin_C" (`self.GetTransform` (`|GetArrayItem` (`self.SpawnPoint`) (`KismetMathLibrary.RandomIntegerInRange` 0 (- (`KismetArrayLibrary.Array_Length` (`self.SpawnPoint`)) 1)))) "AdjustIfPossibleButDontSpawnIfColliding" "OverrideRootScale" null null))

(fn `UserConstructionScript`)